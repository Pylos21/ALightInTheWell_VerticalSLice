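; Key card pickup that adds its KeyChannel to the player's BP_ThirdPersonCharacter when collected.
; Sphere overlap with that character shows a PickUpKey prompt widget, turns on the card's Highlight material parameter and opens a Gate; leaving reverses all three.
; The actor enables input on BeginPlay, and Interact only passes while the Gate is open, playing a sound, granting the key and destroying the card.
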(event `self.ReceiveBeginPlay`
  ;[1 1 1] Enables Input
  (`self.EnableInput` (`GameplayStatics.GetPlayerController` 0)))

(event `InputAction|Interact` :consume false
  (params (Key :type "Key Structure"))
  (:`Pressed`
    (`/Engine/EditorBlueprintResources/StandardMacros.Gate` true :!label _label
      (:`Exit`
        (`GameplayStatics.PlaySoundAtLocation` null (0.0 0.0 0.0) (struct) 1.0 1.0 0.0 null null null null)
        (`/Game/ThirdPerson/Blueprints/BP_ThirdPersonCharacter.AddKey` (cast `/Game/ThirdPerson/Blueprints/BP_ThirdPersonCharacter` (`GameplayStatics.GetPlayerCharacter` 0) :!pure true) (`self.KeyChannel`))
        (`self.K2_DestroyActor`)))))

(event `self.Sphere.OnComponentBeginOverlap`
  (params (OverlappedComponent :type "PrimitiveComponent Object Reference") (OtherActor :type "Actor Object Reference") (OtherComp :type "PrimitiveComponent Object Reference") (OtherBodyIndex :type Integer) (bFromSweep :type Boolean) (SweepResult :type "HitResult Structure (by ref)"))
  (cast `/Game/ThirdPerson/Blueprints/BP_ThirdPersonCharacter` OtherActor)
  (bind _returnvalue (`|CreateWidget` "/Game/ALightInTheWell/Widgets/Interaction/PickUpKey.PickUpKey_C"))
  (`UserWidget.AddToViewport` _returnvalue 0)
  (`MeshComponent.SetScalarParameterValueOnMaterials` (`self.Card`) "Highlight" 1.0)
  (goto _label :!via `Open`))

(event `self.Sphere.OnComponentEndOverlap`
  (params (OverlappedComponent :type "PrimitiveComponent Object Reference") (OtherActor :type "Actor Object Reference") (OtherComp :type "PrimitiveComponent Object Reference") (OtherBodyIndex :type Integer))
  (cast `/Game/ThirdPerson/Blueprints/BP_ThirdPersonCharacter` OtherActor)
  (`Widget.RemoveFromParent` (stale `self.Sphere.OnComponentBeginOverlap` _returnvalue))
  (`MeshComponent.SetScalarParameterValueOnMaterials` (`self.Card`) "Highlight" 0.0)
  (goto _label :!via `Close`))

(fn `UserConstructionScript`)