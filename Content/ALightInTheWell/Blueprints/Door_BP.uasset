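; Card-locked door that the player opens with Interact while inside its trigger box, provided the first linked SwipeCards_BP1 reader has been swiped.
; A gate driven by third-person character overlaps filters the input.
; Timelines lerp door yaw and handle roll.
; Delays chained from timeline updates auto-close the door, then turn the reader's light and material red and clear its Green and the door's IsOpen flags.
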(event `self.ReceiveBeginPlay`
  ;[1 1 1] Enables Input
  (`self.EnableInput` (`GameplayStatics.GetPlayerController` 0)))

(event `InputAction|Interact` :consume false
  (params (Key :type "Key Structure"))
  (bind _asswipe_cards_bp1 (cast `/Game/ALightInTheWell/Blueprints/SwipeCards_BP1` (`|GetArrayItem` (`self.Swipe Cards`)) :!pure true))
  ;[1 1 1] Interact
  (:`Pressed`
    (`/Engine/EditorBlueprintResources/StandardMacros.Gate` true :!label _label
      (:`Exit`
        ;[1 1 1] DoorSystem
        (if (`/Game/ALightInTheWell/Blueprints/SwipeCards_BP1.Swiped?` _asswipe_cards_bp1)
          (if (not (`self.isOpen?`))
            (`|ExecutionSequence`
              (:`then_0`
                (bind (_direction _dooropen) (`Timeline|OpenDoor` :!via `PlayFromStart`)
                  (:`Update`
                    (`SceneComponent.K2_SetRelativeRotation` (`self.Pivot`) (`KismetMathLibrary.MakeRotator` 0.0 0.0 (`KismetMathLibrary.Lerp` (`self.DoorCloseFloat`) (`self.DoorOpenFloat`) _dooropen)) false false))))
              (:`then_1`
                (bind (_direction_2 _dooropen_2) (`Timeline|HandleOpen` :!via `PlayFromStart`)
                  (:`Update`
                    (`SceneComponent.K2_SetRelativeRotation` (`self.Handle_Pivot`) (`KismetMathLibrary.MakeRotator` (`KismetMathLibrary.Lerp` (`self.HandleClosing`) (`self.HandleOpening`) _dooropen_2)) false false)))))
            (set `self.isOpen?` true)
            (`KismetSystemLibrary.Delay` 3.4)
            (bind (_direction_3 _dooropen_3) (`Timeline|CloseDoor` :!via `ReverseFromEnd`)
              (:`Update`
                (`SceneComponent.K2_SetRelativeRotation` (`self.Pivot`) (`KismetMathLibrary.MakeRotator` 0.0 0.0 (`KismetMathLibrary.Lerp` (`self.DoorCloseFloat`) (`self.DoorOpenFloat`) _dooropen_3)) false false)
                (`KismetSystemLibrary.Delay` 10.0)
                (`LightComponent.SetLightColor` (`/Game/ALightInTheWell/Blueprints/SwipeCards_BP1.Light` _asswipe_cards_bp1) (struct :`R` 1.0 :`A` 1.0) true)
                (`PrimitiveComponent.SetMaterial` (`/Game/ALightInTheWell/Blueprints/SwipeCards_BP1.SwipeCards` _asswipe_cards_bp1) 0 "/Game/ALightInTheWell/Environment/Materials/Materials/General/Glow_Red.Glow_Red")
                (set `/Game/ALightInTheWell/Blueprints/SwipeCards_BP1.Green?` false _asswipe_cards_bp1)
                (set `self.isOpen?` false)))))))))

(event `self.Box.OnComponentBeginOverlap`
  (params (OverlappedComponent :type "PrimitiveComponent Object Reference") (OtherActor :type "Actor Object Reference") (OtherComp :type "PrimitiveComponent Object Reference") (OtherBodyIndex :type Integer) (bFromSweep :type Boolean) (SweepResult :type "HitResult Structure (by ref)"))
  ;[1 1 1] Interact
  (cast `/Game/ThirdPerson/Blueprints/BP_ThirdPersonCharacter` OtherActor)
  (goto _label :!via `Open`))

(event `self.Box.OnComponentEndOverlap`
  (params (OverlappedComponent :type "PrimitiveComponent Object Reference") (OtherActor :type "Actor Object Reference") (OtherComp :type "PrimitiveComponent Object Reference") (OtherBodyIndex :type Integer))
  ;[1 1 1] Interact
  (cast `/Game/ThirdPerson/Blueprints/BP_ThirdPersonCharacter` OtherActor)
  (goto _label :!via `Close`))

(fn `UserConstructionScript`)