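; Keycard reader actor that turns green when the player swipes with a key matching its KeyChannel.
; Its box overlap shows a keycard-required widget and opens a gate for the Interact response.
; After a short delay it sets Swiped, plays a sound and turns the light and material green.
; Seven seconds later it clears Swiped, reverting to red if the first linked Door_BP is not open.
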(event `self.ReceiveBeginPlay`
  ;[1 1 1] Enables Input
  (`self.EnableInput` (`GameplayStatics.GetPlayerController` 0)))

(event `InputAction|Interact` :consume false
  (params (Key :type "Key Structure"))
  ;[1 1 1] Interact
  (:`Pressed`
    (if (`self.CanSwipe?`)
      (`GameplayStatics.PlaySoundAtLocation` null (0.0 0.0 0.0) (struct) 1.0 1.0 0.0 null null null null)
      (`/Engine/EditorBlueprintResources/StandardMacros.Gate` true :!label _label
        (:`Exit`
          (`KismetSystemLibrary.Delay` 0.5)
          (set `self.Swiped?` true)
          (`GameplayStatics.PlaySound2D` null 1.0 1.0 0.0 null null)
          (`LightComponent.SetLightColor` (`self.Light`) (struct :`G` 0.717647 :`B` 0.027451 :`A` 1.0) true)
          (`PrimitiveComponent.SetMaterial` (`self.SwipeCards`) 0 "/Game/ALightInTheWell/Environment/Buildings/Materials/General/Glow_Green.Glow_Green")
          (set `self.Green?` true)
          (`KismetSystemLibrary.Delay` 7.0)
          (set `self.Swiped?` false)
          (if (`/Game/ALightInTheWell/Blueprints/Door_BP.isOpen?` (cast `/Game/ALightInTheWell/Blueprints/Door_BP` (`|GetArrayItem` (`self.Door_BP`)) :!pure true))
            _
            (elif (`self.Green?`)
              (`LightComponent.SetLightColor` (`self.Light`) (struct :`R` 1.0 :`A` 1.0) true)
              (`PrimitiveComponent.SetMaterial` (`self.SwipeCards`) 0 "/Game/ALightInTheWell/Environment/Buildings/Materials/General/Glow_Red.Glow_Red")))))
      (else
        (`GameplayStatics.PlaySoundAtLocation` null (0.0 0.0 0.0) (struct) 1.0 1.0 0.0 null null null null)))))

(event `self.Box.OnComponentBeginOverlap`
  (params (OverlappedComponent :type "PrimitiveComponent Object Reference") (OtherActor :type "Actor Object Reference") (OtherComp :type "PrimitiveComponent Object Reference") (OtherBodyIndex :type Integer) (bFromSweep :type Boolean) (SweepResult :type "HitResult Structure (by ref)"))
  ;[1 1 1] Interact
  (cast `/Game/ThirdPerson/Blueprints/BP_ThirdPersonCharacter` OtherActor)
  (bind _returnvalue (`|CreateWidget` "/Game/ALightInTheWell/Widgets/Interaction/KeyCardForOfficeRequired.KeyCardForOfficeRequired_C"))
  (`UserWidget.AddToViewport` _returnvalue 0)
  (goto _label :!via `Open`))

(event `self.Box.OnComponentEndOverlap`
  (params (OverlappedComponent :type "PrimitiveComponent Object Reference") (OtherActor :type "Actor Object Reference") (OtherComp :type "PrimitiveComponent Object Reference") (OtherBodyIndex :type Integer))
  ;[1 1 1] Interact
  (cast `/Game/ThirdPerson/Blueprints/BP_ThirdPersonCharacter` OtherActor)
  (`Widget.RemoveFromParent` (stale `self.Box.OnComponentBeginOverlap` _returnvalue))
  (goto _label :!via `Close`))

(fn `CanSwipe?`
  (returns (`HasKey?` :type Boolean))
  (return (`/Game/ThirdPerson/Blueprints/BP_ThirdPersonCharacter.HasKey` (cast `/Game/ThirdPerson/Blueprints/BP_ThirdPersonCharacter` (`GameplayStatics.GetPlayerCharacter` 0) :!pure true) (`self.KeyChannel`))))

(fn `UserConstructionScript`)