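; Door Blueprint that swings open on its Pivot when the player presses Interact nearby and either linked swipe card reader is swiped.
; A Gate opened by box overlap filters the input, and a sound plays before the swipe check.
; Timelines lerp the yaw open, then closed after a short delay.
; A further delay turns both readers red, clears their Green flags and resets IsOpen.
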(event `self.ReceiveBeginPlay`
  ;[1 1 1] Enables Input
  (`self.EnableInput` (`GameplayStatics.GetPlayerController` 0)))

(event `InputAction|Interact` :consume false
  (params (Key :type "Key Structure"))
  (bind _asswipe_cards_double_door_bp (cast `/Game/ALightInTheWell/Blueprints/SwipeCardsDoubleDoor_BP` (`|GetArrayItem` (`self.SwipeCards`)) :!pure true))
  ;[1 1 1] Interact
  (:`Pressed`
    (`/Engine/EditorBlueprintResources/StandardMacros.Gate` true :!label _label
      (:`Exit`
        ;[1 1 1] DoorSystem
        (`GameplayStatics.PlaySound2D` null 1.0 1.0 0.0 null null)
        (if (`self.SwipeGreen?`)
          (if (not (`self.IsOpen?`))
            (bind (_direction _dooropen) (`Timeline|DoorOpen` :!via `PlayFromStart`)
              (:`Update`
                (`SceneComponent.K2_SetRelativeRotation` (`self.Pivot`) (`KismetMathLibrary.MakeRotator` 0.0 0.0 (`KismetMathLibrary.Lerp` (`self.DoorCloseFloat`) (`self.DoorOpenFloat`) _dooropen)) false false)
                (set `self.IsOpen?` true)
                (`KismetSystemLibrary.Delay` 2.0)
                (bind (_direction_2 _dooropen_2) (`Timeline|DoorClose` :!via `ReverseFromEnd`)
                  (:`Update`
                    (`SceneComponent.K2_SetRelativeRotation` (`self.Pivot`) (`KismetMathLibrary.MakeRotator` 0.0 0.0 (`KismetMathLibrary.Lerp` (`self.DoorCloseFloat`) (`self.DoorOpenFloat`) _dooropen_2)) false false)
                    (`KismetSystemLibrary.Delay` 10.0)
                    (`LightComponent.SetLightColor` (`/Game/ALightInTheWell/Blueprints/SwipeCardsDoubleDoor_BP.Light` _asswipe_cards_double_door_bp) (struct :`R` 1.0 :`A` 1.0) true)
                    (`LightComponent.SetLightColor` (`/Game/ALightInTheWell/Blueprints/SwipeCardsDoubleDoor_BP.Light` (cast `/Game/ALightInTheWell/Blueprints/SwipeCardsDoubleDoor_BP` (`|GetArrayItem` (`self.SwipeCards`) 1) :!pure true)) (struct :`R` 1.0 :`A` 1.0) true)
                    (`PrimitiveComponent.SetMaterial` (`/Game/ALightInTheWell/Blueprints/SwipeCardsDoubleDoor_BP.SwipeCards` _asswipe_cards_double_door_bp) 0 "/Game/ALightInTheWell/Environment/Materials/Materials/General/Glow_Red.Glow_Red")
                    (`PrimitiveComponent.SetMaterial` (`/Game/ALightInTheWell/Blueprints/SwipeCardsDoubleDoor_BP.SwipeCards` (cast `/Game/ALightInTheWell/Blueprints/SwipeCardsDoubleDoor_BP` (`|GetArrayItem` (`self.SwipeCards`) 1) :!pure true)) 0 "/Game/ALightInTheWell/Environment/Materials/Materials/General/Glow_Red.Glow_Red")
                    (set `/Game/ALightInTheWell/Blueprints/SwipeCardsDoubleDoor_BP.Green?` false _asswipe_cards_double_door_bp)
                    (set `/Game/ALightInTheWell/Blueprints/SwipeCardsDoubleDoor_BP.Green?` false (cast `/Game/ALightInTheWell/Blueprints/SwipeCardsDoubleDoor_BP` (`|GetArrayItem` (`self.SwipeCards`) 1) :!pure true))
                    (set `self.IsOpen?` false)))))))))))

(event `self.Box.OnComponentBeginOverlap`
  (params (OverlappedComponent :type "PrimitiveComponent Object Reference") (OtherActor :type "Actor Object Reference") (OtherComp :type "PrimitiveComponent Object Reference") (OtherBodyIndex :type Integer) (bFromSweep :type Boolean) (SweepResult :type "HitResult Structure (by ref)"))
  ;[1 1 1] Interact
  (cast `/Game/ThirdPerson/Blueprints/BP_ThirdPersonCharacter` OtherActor)
  (goto _label :!via `Open`))

(event `self.Box.OnComponentEndOverlap`
  (params (OverlappedComponent :type "PrimitiveComponent Object Reference") (OtherActor :type "Actor Object Reference") (OtherComp :type "PrimitiveComponent Object Reference") (OtherBodyIndex :type Integer))
  ;[1 1 1] Interact
  (cast `/Game/ThirdPerson/Blueprints/BP_ThirdPersonCharacter` OtherActor)
  (goto _label :!via `Close`))

(fn `SwipeGreen?`
  (returns (ReturnValue :type Boolean))
  (return (or (`/Game/ALightInTheWell/Blueprints/SwipeCardsDoubleDoor_BP.Swiped?` (cast `/Game/ALightInTheWell/Blueprints/SwipeCardsDoubleDoor_BP` (`|GetArrayItem` (`self.SwipeCards`)) :!pure true)) (`/Game/ALightInTheWell/Blueprints/SwipeCardsDoubleDoor_BP.Swiped?` (cast `/Game/ALightInTheWell/Blueprints/SwipeCardsDoubleDoor_BP` (`|GetArrayItem` (`self.SwipeCards`) 1) :!pure true)))))

(fn `UserConstructionScript`)